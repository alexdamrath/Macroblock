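; Player character with camera-relative movement on three axes and a chargeable punch that launches it forward.
; Holding Fire without a gun runs a timeline that builds punch force and widens the FOV.
; Releasing Fire, gun or not, applies that force as an impulse along the camera, resets FOV and sets Punching.
; Hits deal damage while Punching, which is never cleared here; BeginPlay also creates the HUD.
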(event EventBeginPlay
  (bind _returnvalue (UserInterface|CreateWidget "/Game/Blueprints/HUD.HUD_C" (Game|GetPlayerController 0)))
  (bind _output_get (Variables|Default|SetHUD _returnvalue))
  (UserInterface|Viewport|AddtoPlayerScreen _output_get))

(event Collision|EventHit
  (params (MyComp :type Primitive%20Component%20Object%20Reference) (Other :type Actor%20Object%20Reference) (OtherComp :type Primitive%20Component%20Object%20Reference) (bSelfMoved :type Boolean) (HitLocation :type Vector :default "0, 0, 0") (HitNormal :type Vector :default "0, 0, 0") (NormalImpulse :type Vector :default "0, 0, 0") (Hit :type Hit%20Result%20Structure%20%28by%20ref%29))
  (if (Variables|Default|GetPunching)
    (Game|Damage|ApplyDamage Other 1.0 0 0)))

(event Input|ActionEvents|InputActionFire
  (params (Key :type Key%20Structure))
  (bind _camera (Variables|Default|GetCamera))
  (:Pressed
    (if (not (Variables|Default|GetHasGun))
      (bind _charge (Timeline|PunchCharge PlayFromStart)
        (:Update
          (Variables|Default|SetPunchForce (Math|Float|Lerp 0.0 1.0 _charge))
          (Camera|SetFieldOfView _camera (Math|Float|Lerp 9e+01 98.0 _charge))))))
  (:Released
    (Utilities|FlowControl|Sequence
      (:then_0
        (Timeline|PunchCharge Stop))
      (:then_1
        (Physics|AddImpulse (Variables|Character|GetCharacterMovement) (* (Math|Vector|GetForwardVector (Variables|Default|GetCamera)) (* 3e+03 (Variables|Default|GetPunchForce))) true)
        (Variables|Default|SetPunchForce 0.0)
        (Camera|SetFieldOfView _camera 9e+01)
        (Variables|Default|SetPunching true)
        (Development|PrintString "PUNCH")
        (Utilities|FlowControl|Delay 0.5)
        (Development|PrintString "NO PUNCH")))))

(event Input|AxisEvents|InputAxisLookUp
  (params (AxisValue :type Float%20%28single-precision%29))
  (Pawn|Input|AddControllerPitchInput AxisValue))

(event Input|AxisEvents|InputAxisForward
  (params (AxisValue :type Float%20%28single-precision%29))
  (Pawn|Input|AddMovementInput (Math|Vector|GetForwardVector (Variables|Default|GetCamera)) AxisValue false))

(event Input|AxisEvents|InputAxisRight
  (params (AxisValue :type Float%20%28single-precision%29))
  (Pawn|Input|AddMovementInput (Math|Vector|GetRightVector (Variables|Default|GetCamera)) AxisValue false))

(event Input|AxisEvents|InputAxisUp
  (params (AxisValue :type Float%20%28single-precision%29))
  (Pawn|Input|AddMovementInput (Math|Vector|GetUpVector (Variables|Default|GetCamera)) AxisValue false))

(event Input|AxisEvents|InputAxisLookRight
  (params (AxisValue :type Float%20%28single-precision%29))
  (Pawn|Input|AddControllerYawInput AxisValue))

(fn ConstructionScript)