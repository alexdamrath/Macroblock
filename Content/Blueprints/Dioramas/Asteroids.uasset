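; Asteroids diorama Blueprint meant to scatter asteroid actors, but its BeginPlay and construction script are empty.
; An unconnected loop would spawn Asteroid actors with random location, rotation and per-axis scale, printing a debug message for each.
; Spawn points come from the bounds of the physics volume returned by the Box component, rather than the box's own extent.
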(event EventBeginPlay)

(fn ConstructionScript)