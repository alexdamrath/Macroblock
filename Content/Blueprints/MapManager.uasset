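; MapManager is a Blueprint that rolls a weighted container tier once at BeginPlay.
; A single random integer passes through cascading threshold branches to pick SAFE, CRATE, CARD or OPEN, with SAFE the most likely and OPEN the least.
; The chosen tier is only printed as a debug string; nothing is spawned, and the construction script is empty.
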(event EventBeginPlay
  (bind _output_get (Variables|Default|SetContainerTierSelector (Math|Random|RandomInteger 100)))
  (if (<= _output_get 50)
    (Development|PrintString "SAFE")
    (elif (<= _output_get 75)
      (Development|PrintString "CRATE")
      (elif (<= _output_get 90)
        (Development|PrintString "CARD")
        (else
          (Development|PrintString "OPEN"))))))

(fn ConstructionScript)