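; Wall actor made of four cube components that takes on a randomly chosen layout when play begins.
; The construction script gathers the cubes into an array.
; BeginPlay rolls one index from the first cube's transform list and uses it for every cube, each reading its own transform array, so the offsets form matched sets.
; Each chosen transform is added as a local offset without sweep.
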(event EventBeginPlay
  (Variables|Default|SetSet# (Math|Random|RandomInteger (Utilities|Array|Length (Variables|Default|GetCube1_Tsets))))
  (for (_array_element _array_index) (Variables|Default|GetWalls)
    (Class|SceneComponent|AddLocalTransform _array_element (Utilities|Array|Get(acopy) (Utilities|Select :Index _array_index :Option%200 (Variables|Default|GetCube1_Tsets) :Option%201 (Variables|Default|GetCube2_Tsets) :Option%202 (Variables|Default|GetCube3_Tsets) :Option%203 (Variables|Default|GetCube4_Tsets)) (Variables|Default|GetSet#)) false false)))

(fn ConstructionScript
  (Variables|Default|SetWalls (Utilities|Array|MakeArray (Variables|Default|GetCube1) (Variables|Default|GetCube2) (Variables|Default|GetCube3) (Variables|Default|GetCube4))))